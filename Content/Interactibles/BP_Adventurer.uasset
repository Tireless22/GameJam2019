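; BP_Adventurer is an interactable adventurer that the player-controlled TopDownCharacter can pick up and carry.
; On Interact it sets the character's Carrying flag and snaps onto the mesh's right-hand item socket.
; It then unregisters itself as an interactable, deactivates and disables collision on its area and mesh.
; Ragdoll physics nodes using a locked physics asset are present but never run.
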(event `self.ReceiveBeginPlay`)

(event `Interact`
  (bind _astop_down_character (cast `/Game/TopDownBP/Blueprints/TopDownCharacter` (`Controller.K2_GetPawn` (`GameplayStatics.GetPlayerController` 0))))
  (set `/Game/TopDownBP/Blueprints/TopDownCharacter.Carrying?` true _astop_down_character)
  (`self.K2_AttachToComponent` (`Character.Mesh` _astop_down_character) "RightHand_ItemJoint" "SnapToTarget" "SnapToTarget" "SnapToTarget")
  (`/Game/TopDownBP/Blueprints/TopDownCharacter.Unregister_Interactable` _astop_down_character self)
  (set `self.IsActive?` false)
  (`PrimitiveComponent.SetCollisionEnabled` (`self.InteractableArea`) "NoCollision")
  (`PrimitiveComponent.SetCollisionEnabled` (`self.InteractableMesh`) "NoCollision"))

(fn `UserConstructionScript`
  (`parent.UserConstructionScript`))