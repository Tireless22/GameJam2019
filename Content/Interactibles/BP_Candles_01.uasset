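; Interactable candle cluster that starts unlit and lights up once when interacted with.
; On BeginPlay it switches off the flames and point light, including flames in candle child actors reached by casting to each variant, and gathers them into effect and light arrays.
; Interact activates those effects, shows the light, then clears its active flag, unregisters from the TopDownCharacter and disables the interaction area's collision.
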(event `self.ReceiveBeginPlay`
  (bind _pointlight (`self.PointLight`))
  (`|ExecutionSequence`
    (:`then_0`
      (`ActorComponent.Deactivate` _pointlight)
      (`ActorComponent.Deactivate` (`self.ParticleSystem2`))
      (`ActorComponent.Deactivate` (`self.ParticleSystem1`))
      (`ActorComponent.Deactivate` (`self.ParticleSystem`))
      (`SceneComponent.SetVisibility` _pointlight false false))
    (:`then_1`
      (bind _ascandles_02 (cast `/Game/MultistoryDungeons/Blueprints/Props/Candles_02` (`ChildActorComponent.ChildActor` (`self.ChildActor`))))
      (bind _particlesystem (`/Game/MultistoryDungeons/Blueprints/Props/Candles_02.ParticleSystem` _ascandles_02))
      (`ActorComponent.Deactivate` _particlesystem)
      (`ActorComponent.Deactivate` (`/Game/MultistoryDungeons/Blueprints/Props/Candles_02.ParticleSystem1` _ascandles_02))
      (`ActorComponent.Deactivate` (`/Game/MultistoryDungeons/Blueprints/Props/Candles_02.ParticleSystem2` _ascandles_02))
      (`ActorComponent.Deactivate` (`/Game/MultistoryDungeons/Blueprints/Props/Candles_02.ParticleSystem3` _ascandles_02)))
    (:`then_2`
      (bind _ascandles_03 (cast `/Game/MultistoryDungeons/Blueprints/Props/Candles_03` (`ChildActorComponent.ChildActor` (`self.ChildActor1`))))
      (bind _particlesystem1 (`/Game/MultistoryDungeons/Blueprints/Props/Candles_03.ParticleSystem1` _ascandles_03))
      (`ActorComponent.Deactivate` _particlesystem1)
      (`ActorComponent.Deactivate` (`/Game/MultistoryDungeons/Blueprints/Props/Candles_03.ParticleSystem2` _ascandles_03))
      (`ActorComponent.Deactivate` (`/Game/MultistoryDungeons/Blueprints/Props/Candles_03.ParticleSystem` _ascandles_03)))
    (:`then_3`
      (bind _ascandles_04 (cast `/Game/MultistoryDungeons/Blueprints/Props/Candles_04` (`ChildActorComponent.ChildActor` (`self.ChildActor2`))))
      (bind _particlesystem1_2 (`/Game/MultistoryDungeons/Blueprints/Props/Candles_04.ParticleSystem1` _ascandles_04))
      (`ActorComponent.Deactivate` _particlesystem1_2)
      (`ActorComponent.Deactivate` (`/Game/MultistoryDungeons/Blueprints/Props/Candles_04.ParticleSystem` _ascandles_04)))
    (:`then_4`
      (bind _ascandles_05 (cast `/Game/MultistoryDungeons/Blueprints/Props/Candles_05` (`ChildActorComponent.ChildActor` (`self.ChildActor3`))))
      (bind _particlesystem_2 (`/Game/MultistoryDungeons/Blueprints/Props/Candles_05.ParticleSystem` _ascandles_05))
      (`ActorComponent.Deactivate` _particlesystem_2))
    (:`then_5`
      (set `self.FXArray` (`|MakeArray` (`self.ParticleSystem`) (`self.ParticleSystem1`) (`self.ParticleSystem2`) _particlesystem (`/Game/MultistoryDungeons/Blueprints/Props/Candles_02.ParticleSystem1` _ascandles_02) (`/Game/MultistoryDungeons/Blueprints/Props/Candles_02.ParticleSystem2` _ascandles_02) (`/Game/MultistoryDungeons/Blueprints/Props/Candles_02.ParticleSystem3` _ascandles_02) _particlesystem1 (`/Game/MultistoryDungeons/Blueprints/Props/Candles_03.ParticleSystem2` _ascandles_03) (`/Game/MultistoryDungeons/Blueprints/Props/Candles_03.ParticleSystem` _ascandles_03) (`/Game/MultistoryDungeons/Blueprints/Props/Candles_04.ParticleSystem` _ascandles_04) _particlesystem1_2 _particlesystem_2))
      (set `self.LightArray` (`|MakeArray` _pointlight)))
    (:`then_6`
      (for _array_element (`|MakeArray` (`ChildActorComponent.ChildActor` (`self.ChildActor4`)) (`ChildActorComponent.ChildActor` (`self.ChildActor5`)))
        (bind _ascandles_02_2 (cast `/Game/MultistoryDungeons/Blueprints/Props/Candles_02` _array_element))
        (bind _particlesystem_3 (`/Game/MultistoryDungeons/Blueprints/Props/Candles_02.ParticleSystem` _ascandles_02_2))
        (`ActorComponent.Deactivate` _particlesystem_3)
        (`ActorComponent.Deactivate` (`/Game/MultistoryDungeons/Blueprints/Props/Candles_02.ParticleSystem1` _ascandles_02_2))
        (`ActorComponent.Deactivate` (`/Game/MultistoryDungeons/Blueprints/Props/Candles_02.ParticleSystem2` _ascandles_02_2))
        (`ActorComponent.Deactivate` (`/Game/MultistoryDungeons/Blueprints/Props/Candles_02.ParticleSystem3` _ascandles_02_2))
        (for _array_element_2 (`|MakeArray` _particlesystem_3 (`/Game/MultistoryDungeons/Blueprints/Props/Candles_02.ParticleSystem1` _ascandles_02_2) (`/Game/MultistoryDungeons/Blueprints/Props/Candles_02.ParticleSystem2` _ascandles_02_2) (`/Game/MultistoryDungeons/Blueprints/Props/Candles_02.ParticleSystem3` _ascandles_02_2))
          (`KismetArrayLibrary.Array_Add` (`self.FXArray`) _array_element_2)))
      (for _array_element_3 (`|MakeArray` (`ChildActorComponent.ChildActor` (`self.ChildActor6`)) (`ChildActorComponent.ChildActor` (`self.ChildActor7`)))
        (bind _ascandles_04_2 (cast `/Game/MultistoryDungeons/Blueprints/Props/Candles_04` _array_element_3))
        (bind _particlesystem1_3 (`/Game/MultistoryDungeons/Blueprints/Props/Candles_04.ParticleSystem1` _ascandles_04_2))
        (`ActorComponent.Deactivate` _particlesystem1_3)
        (`ActorComponent.Deactivate` (`/Game/MultistoryDungeons/Blueprints/Props/Candles_04.ParticleSystem` _ascandles_04_2))
        (for _array_element_4 (`|MakeArray` (`/Game/MultistoryDungeons/Blueprints/Props/Candles_04.ParticleSystem` _ascandles_04_2) _particlesystem1_3)
          (`KismetArrayLibrary.Array_Add` (`self.FXArray`) _array_element_4))))))

(event `Interact`
  (set `self.IsActive?` false)
  (for _array_element (`self.FXArray`)
    (`ActorComponent.Activate` _array_element false))
  (for _array_element_2 (`self.LightArray`)
    (`SceneComponent.SetVisibility` _array_element_2 true false))
  (`/Game/TopDownBP/Blueprints/TopDownCharacter.Unregister_Interactable` (cast `/Game/TopDownBP/Blueprints/TopDownCharacter` (`GameplayStatics.GetPlayerCharacter` 0) :!pure true) self)
  (`PrimitiveComponent.SetCollisionEnabled` (`self.InteractableArea`) "NoCollision"))

(fn `UserConstructionScript`
  (`parent.UserConstructionScript`))