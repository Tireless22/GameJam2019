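; BP_Walltorch is an interactable wall torch that the player can light.
; On Interact, it checks the TopDownCharacter's TorchOut flag; if set, it activates the fire effect and shows the point light.
; It then sets IsActive false, unregisters itself from the character and disables the interact area's collision, making lighting a one-time action.
; Without a torch out, it prints a flavor hint instead.
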(event `Interact`
  (bind _astop_down_character (cast `/Game/TopDownBP/Blueprints/TopDownCharacter` (`GameplayStatics.GetPlayerCharacter` 0)))
  (if (`/Game/TopDownBP/Blueprints/TopDownCharacter.TorchOut?` _astop_down_character)
    (`ActorComponent.SetActive` (`self.Fire`) true false)
    (`SceneComponent.SetVisibility` (`self.PointLight`) true false)
    (set `self.IsActive?` false)
    (bind _astop_down_character_2 (cast `/Game/TopDownBP/Blueprints/TopDownCharacter` (`GameplayStatics.GetPlayerCharacter` 0)))
    (`/Game/TopDownBP/Blueprints/TopDownCharacter.Unregister_Interactable` _astop_down_character_2 self)
    (`PrimitiveComponent.SetCollisionEnabled` (`self.InteractableArea`) "NoCollision")
    (else
      (`KismetSystemLibrary.PrintString` "I should probably light these to set the mood for the next Adventurer..."))))

(fn `UserConstructionScript`
  (`parent.UserConstructionScript`))