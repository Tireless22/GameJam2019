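; Interactible fade plane that toggles its static mesh between opaque and transparent, apparently to hide or reveal a dungeon area.
; On BeginPlay it creates a dynamic instance of the fading material at full opacity.
; ToggleVisible starts a fast looping timer on FadeOut, which, despite its name, steps opacity up or down depending on DungeonIsHidden.
; At either limit it clamps the value, clears the timer and flips the flag.
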(event `self.ReceiveBeginPlay`
  (bind _returnvalue (`PrimitiveComponent.CreateDynamicMaterialInstance` (`self.StaticMesh`) 0 "/Game/Assets/Materials/fading_material_Inst.fading_material_Inst" "None"))
  (set `self.dungeon_mat` _returnvalue)
  (`MaterialInstanceDynamic.SetScalarParameterValue` (`self.dungeon_mat`) "opacity" 1.0))

(event `ToggleVisible`
  (bind _returnvalue (`KismetSystemLibrary.K2_SetTimerDelegate` (delegate `FadeOut`) 0.01 true))
  (set `self.DungeonHandle` _returnvalue))

(event `FadeOut`
  (if (`self.DungeonIsHidden?`)
    ;[1 1 1] increase till 1
    (set `self.Float` (+ (`self.Float`) 0.01))
    (if (>= (`self.Float`) 1.0)
      (set `self.Float` 1.0)
      (`KismetSystemLibrary.K2_ClearAndInvalidateTimerHandle` (`self.DungeonHandle`))
      (`MaterialInstanceDynamic.SetScalarParameterValue` (`self.dungeon_mat`) "opacity" (`self.Float`))
      (set `self.DungeonIsHidden?` false)
      (else
        (`MaterialInstanceDynamic.SetScalarParameterValue` (`self.dungeon_mat`) "opacity" (`self.Float`))))
    (else
      ;[1 1 1] decrease till 0
      (set `self.Float` (- (`self.Float`) 0.01))
      (if (<= (`self.Float`) 0.0)
        (set `self.Float` 0.0)
        (`KismetSystemLibrary.K2_ClearAndInvalidateTimerHandle` (`self.DungeonHandle`))
        (`MaterialInstanceDynamic.SetScalarParameterValue` (`self.dungeon_mat`) "opacity" (`self.Float`))
        (set `self.DungeonIsHidden?` true)
        (else
          (`MaterialInstanceDynamic.SetScalarParameterValue` (`self.dungeon_mat`) "opacity" (`self.Float`)))))))

(fn `UserConstructionScript`)