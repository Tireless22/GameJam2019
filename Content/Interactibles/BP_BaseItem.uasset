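; BP_BaseItem is a base interactible item Blueprint that defines pickup behavior and carries an ItemInfo struct.
; Its construction script calls the parent, then rebuilds ItemInfo with the actor's own class, keeping the other listed fields.
; The Interaction event holds pickup logic that passes ItemInfo to the instigator, plays a plop sound and destroys the actor.
; That logic sits behind a constant-false branch, so it never runs here.
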(event `/Game/Interactibles/BPI_Interact.Interaction`
  (params (Instigator :type "/Game/TopDownBP/Blueprints/TopDownCharacter Object Reference"))
  (if false
    (message `/Game/Interactibles/BPI_Interact.Pickup` Instigator (`self.ItemInfo`))
    (`GameplayStatics.PlaySound2D` "/Game/SFX/cue_plop.cue_plop" 1.0 1.0 0.0 null null)
    (`self.K2_DestroyActor`)))

(fn `UserConstructionScript`
  (bind (_iteminfo_itemtype _iteminfo_itemname _iteminfo_itemimage _iteminfo_itemclass _iteminfo_itemindex _iteminfo_itemslot _iteminfo_itemvalue _iteminfo_stackable_ _iteminfo_stacksize _iteminfo_maxstacksize) (break `/Game/Interactibles/F_Item_Info` (`self.ItemInfo`)))
  (`parent.UserConstructionScript`)
  (set `self.ItemInfo` (make `/Game/Interactibles/F_Item_Info` _iteminfo_itemtype _iteminfo_itemname _iteminfo_itemimage (`GameplayStatics.GetObjectClass` self) _iteminfo_itemindex _iteminfo_itemslot _iteminfo_itemvalue _iteminfo_stackable_ _iteminfo_stacksize _iteminfo_maxstacksize)))