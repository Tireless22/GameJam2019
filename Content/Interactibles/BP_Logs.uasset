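; BP_Logs is an interactable pile or item of logs that the player's TopDownCharacter can pick up, carry and drop.
; InteractLogs sets the character's Carrying flag, snaps the logs to its right-hand socket, unregisters them as interactable and disables collision.
; Drop teleports them just in front of the character, detaches them, restores collision, enables mesh physics and reactivates them, without clearing Carrying itself.
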(event `InteractLogs`
  (bind _astop_down_character (cast `/Game/TopDownBP/Blueprints/TopDownCharacter` (`Controller.K2_GetPawn` (`GameplayStatics.GetPlayerController` 0))))
  (set `/Game/TopDownBP/Blueprints/TopDownCharacter.Carrying?` true _astop_down_character)
  (`self.K2_AttachToComponent` (`Character.Mesh` _astop_down_character) "RightHand_ItemJoint" "SnapToTarget" "SnapToTarget" "SnapToTarget")
  (`/Game/TopDownBP/Blueprints/TopDownCharacter.Unregister_Interactable` _astop_down_character self)
  (set `self.IsActive?` false)
  (`PrimitiveComponent.SetCollisionEnabled` (`self.InteractableArea`) "NoCollision")
  (`PrimitiveComponent.SetCollisionEnabled` (`self.InteractableMesh`) "NoCollision"))

(event `Drop`
  (`self.K2_SetActorLocation` (+ (`self.K2_GetActorLocation` (stale `InteractLogs` _astop_down_character)) (* (`SceneComponent.GetForwardVector` (`Actor.RootComponent` (stale `InteractLogs` _astop_down_character))) 50.0)) false true)
  (`self.K2_DetachFromActor` "KeepWorld" "KeepWorld" "KeepWorld")
  (`PrimitiveComponent.SetCollisionEnabled` (`self.InteractableArea`) "QueryAndPhysics")
  (`PrimitiveComponent.SetCollisionEnabled` (`self.InteractableMesh`) "QueryAndPhysics")
  (`PrimitiveComponent.SetSimulatePhysics` (`self.InteractableMesh`) true)
  (set `self.IsActive?` true))

(fn `UserConstructionScript`
  (`parent.UserConstructionScript`))