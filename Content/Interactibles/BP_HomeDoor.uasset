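; Interactable home door, apparently leading to the dungeon, that signals with lights and a spinning wheel when it can be used.
; StartBlinkingSpinngin runs light and wheel timelines with sound, then turns green, enables interaction, registers a nearby player and triggers DoOnce-gated DungeonHandler dialogue chosen by a counter.
; Interact swings the door open, toggles the dungeon fade plane and ramps player walk speed.
; Separate open and close events animate the door and switch light states.
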(event `StartBlinkingSpinngin`
  ;[1 1 1] spin then go green and allow interaction
  (`|ExecutionSequence`
    (:`then_0`
      (bind (_direction _newtrack_0) (`Timeline|Timeline_2` :!via `PlayFromStart`)
        (:`Update`
          (bind _returnvalue (* _newtrack_0 100.0))
          (`LightComponent.SetIntensity` (`self.PointLight1`) _returnvalue)
          (`LightComponent.SetIntensity` (`self.PointLight`) _returnvalue))
        (:`Finished`
          (`self.SetLightGreen`)
          (set `self.IsActive?` true)
          (`PrimitiveComponent.SetCollisionEnabled` (`self.InteractableArea`) "QueryAndPhysics")
          (bind _astop_down_character (cast `/Game/TopDownBP/Blueprints/TopDownCharacter` (`GameplayStatics.GetPlayerCharacter` 0)))
          (if (<= (`KismetMathLibrary.Vector_Distance` (`SceneComponent.K2_GetComponentLocation` (`Character.Mesh` _astop_down_character)) (`SceneComponent.K2_GetComponentLocation` (`self.Scene`))) 180.0)
            (message `/Game/Interactibles/BPI_Interact.RegisterInteractable` _astop_down_character self)
            (`/Engine/EditorBlueprintResources/StandardMacros.DoOnce` false
              (:`Completed`
                (switch `int` (`self.iunt`)
                  (:`0`
                    (bind _outactors (`GameplayStatics.GetAllActorsOfClass` "/Game/Interactibles/DungeonHandler.DungeonHandler_C"))
                    (`/Game/Interactibles/DungeonHandler.StartDialogue` (`|GetArrayItem` _outactors) "Another cleanup requested. Best set the mood for the next Adventurer..."))
                  (:`1`
                    (bind _outactors_2 (`GameplayStatics.GetAllActorsOfClass` "/Game/Interactibles/DungeonHandler.DungeonHandler_C"))
                    (`/Game/Interactibles/DungeonHandler.StartDialogue` (`|GetArrayItem` _outactors_2) "Another fallen Adventurer to clean up... "))
                  (:`2`
                    (bind _outactors_3 (`GameplayStatics.GetAllActorsOfClass` "/Game/Interactibles/DungeonHandler.DungeonHandler_C"))
                    (`/Game/Interactibles/DungeonHandler.StartDialogue` (`|GetArrayItem` _outactors_3) "Ah damn it... I hope the blobs survived...")))
                (`/Engine/EditorBlueprintResources/StandardMacros.IncrementInt` (`self.iunt`))))))))
    (:`then_1`
      (bind _returnvalue_2 (`GameplayStatics.SpawnSound2D` "/Game/SFX/SFX_spinning.SFX_spinning" 1.0 1.0 0.0 null))
      (bind _output_get (set `self.spinningRef` _returnvalue_2))
      (`AudioComponent.FadeIn` _output_get 1.0 1.0 0.0)
      (bind (_direction_2 _newtrack_0_2) (`Timeline|Timeline_3` :!via `PlayFromStart`)
        (:`Update`
          (`SceneComponent.K2_SetWorldRotation` (`self.wheel`) (`KismetMathLibrary.MakeRotator` _newtrack_0_2) false false))
        (:`Finished`
          (`AudioComponent.Stop` (`self.spinningRef`))
          (`GameplayStatics.PlaySound2D` "/Game/SFX/SFX_pling.SFX_pling" 1.0 1.0 0.0 null null))))))

(event `SetLightDefault`
  (bind _pointlight (`self.PointLight`))
  (bind _pointlight1 (`self.PointLight1`))
  ;[1 1 1] set light default
  (`LightComponent.SetIntensity` _pointlight1 50.0)
  (`LightComponent.SetIntensity` _pointlight 50.0)
  (`LightComponent.SetLightColor` _pointlight1 (struct :`R` 0.374642 :`G` 0.613629 :`B` 0.645833 :`A` 1.0) true)
  (`LightComponent.SetLightColor` _pointlight (struct :`R` 0.374642 :`G` 0.613629 :`B` 0.645833 :`A` 1.0) true)
  (`LocalLightComponent.SetAttenuationRadius` _pointlight1 122.0)
  (`LocalLightComponent.SetAttenuationRadius` _pointlight 122.0))

(event `self.ReceiveBeginPlay`
  ;[1 1 1] set references to fade planes on start
  (bind _outactors (`GameplayStatics.GetAllActorsOfClass` "/Game/Interactibles/BP_fadeplane_dungeon.BP_fadeplane_dungeon_C"))
  (set `self.dungeon_fadeplane_ref` (`|GetArrayItem` _outactors))
  (bind _outactors_2 (`GameplayStatics.GetAllActorsOfClass` "/Game/Interactibles/BP_fadeplane_home.BP_fadeplane_home_C"))
  (set `self.home_fadeplane_ref` (`|GetArrayItem` _outactors_2)))

(event `Interact`
  ;[1 1 1] interact and open door
  (`GameplayStatics.PlaySound2D` "/Game/SFX/SFX_opendoor.SFX_opendoor" 1.0 1.0 0.0 null null)
  (`GameplayStatics.PlaySound2D` "/Game/SFX/SFX_door_screetch.SFX_door_screetch" 1.0 1.0 0.0 null null)
  (set `self.IsActive?` false)
  (bind _astop_down_character (cast `/Game/TopDownBP/Blueprints/TopDownCharacter` (`GameplayStatics.GetPlayerCharacter` 0)))
  (`/Game/TopDownBP/Blueprints/TopDownCharacter.Unregister_Interactable` _astop_down_character self)
  (`PrimitiveComponent.SetCollisionEnabled` (`self.InteractableArea`) "NoCollision")
  (`/Game/Interactibles/BP_fadeplane_dungeon.ToggleVisible` (`self.dungeon_fadeplane_ref`))
  (bind (_direction _newtrack_0) (`Timeline|Timeline_0` :!via `PlayFromStart`)
    (:`Update`
      (`self.K2_SetActorRotation` (`KismetMathLibrary.MakeRotator` 0.0 0.0 (`KismetMathLibrary.Lerp` 90.0 180.0 _newtrack_0))))
    (:`Finished`
      ;[1 1 1] Character Speed
      (bind (_direction_2 _newtrack_0_2) (`Timeline|Timeline_5` :!via `PlayFromStart`)
        (:`Update`
          (set `CharacterMovementComponent.MaxWalkSpeed` (`KismetMathLibrary.Lerp` 120.0 450.0 _newtrack_0_2) (`Character.CharacterMovement` (cast `/Game/TopDownBP/Blueprints/TopDownCharacter` (`GameplayStatics.GetPlayerCharacter` 0) :!pure true))))))))

(event `CloseDoor`
  ;[1 1 1] close door
  (`GameplayStatics.PlaySound2D` "/Game/SFX/SFX_door_screetch.SFX_door_screetch" 1.0 1.0 0.0 null null)
  (bind (_direction _newtrack_0) (`Timeline|Timeline_1` :!via `PlayFromStart`)
    (:`Update`
      (`self.K2_SetActorRotation` (`KismetMathLibrary.MakeRotator` 0.0 0.0 (`KismetMathLibrary.Lerp` 180.0 90.0 _newtrack_0)))
      (`self.SetLightDefault`))
    (:`Finished`
      (`GameplayStatics.PlaySound2D` "/Game/SFX/SFX_closedoor.SFX_closedoor" 1.0 1.0 0.0 null null))))

(event `OpenDoor`
  ;[1 1 1] open door
  (`GameplayStatics.PlaySound2D` "/Game/SFX/SFX_opendoor.SFX_opendoor" 1.0 1.0 0.0 null null)
  (`GameplayStatics.PlaySound2D` "/Game/SFX/SFX_door_screetch.SFX_door_screetch" 1.0 1.0 0.0 null null)
  (bind (_direction _newtrack_0) (`Timeline|Timeline_4` :!via `PlayFromStart`)
    (:`Update`
      (`self.K2_SetActorRotation` (`KismetMathLibrary.MakeRotator` 0.0 0.0 (`KismetMathLibrary.Lerp` 90.0 180.0 _newtrack_0))))
    (:`Finished`
      (`self.SetLightGreen`))))

(fn `SetLightGreen`
  (bind _pointlight (`self.PointLight`))
  (bind _pointlight1 (`self.PointLight1`))
  (`LightComponent.SetIntensity` _pointlight1 200.0)
  (`LightComponent.SetIntensity` _pointlight 200.0)
  (`LightComponent.SetLightColor` _pointlight1 (struct :`R` 0.215278 :`G` 0.645833 :`B` 0.291352 :`A` 1.0) true)
  (`LightComponent.SetLightColor` _pointlight (struct :`R` 0.215278 :`G` 0.645833 :`B` 0.291352 :`A` 1.0) true)
  (`LocalLightComponent.SetAttenuationRadius` _pointlight1 300.0)
  (`LocalLightComponent.SetAttenuationRadius` _pointlight 300.0))

(fn `UserConstructionScript`
  (`parent.UserConstructionScript`))