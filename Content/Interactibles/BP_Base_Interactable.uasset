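; Base Blueprint for interactable objects in a top-down game, letting the player character know when one is in range.
; While active, it registers itself with an overlapping TopDownCharacter when that character enters the InteractableArea and unregisters when it leaves.
; SetHighlight toggles custom depth rendering on the interactable mesh to switch its highlight on or off.
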(event `self.InteractableArea.OnComponentBeginOverlap`
  (params (OverlappedComponent :type "PrimitiveComponent Object Reference") (OtherActor :type "Actor Object Reference") (OtherComp :type "PrimitiveComponent Object Reference") (OtherBodyIndex :type Integer) (bFromSweep :type Boolean) (SweepResult :type "HitResult Structure (by ref)"))
  (if (`self.IsActive?`)
    (bind _astop_down_character (cast `/Game/TopDownBP/Blueprints/TopDownCharacter` OtherActor))
    (message `/Game/Interactibles/BPI_Interact.RegisterInteractable` _astop_down_character self)))

(event `self.InteractableArea.OnComponentEndOverlap`
  (params (OverlappedComponent :type "PrimitiveComponent Object Reference") (OtherActor :type "Actor Object Reference") (OtherComp :type "PrimitiveComponent Object Reference") (OtherBodyIndex :type Integer))
  (if (`self.IsActive?`)
    (bind _astop_down_character (cast `/Game/TopDownBP/Blueprints/TopDownCharacter` OtherActor))
    (message `/Game/Interactibles/BPI_Interact.Unregister_Interactable` _astop_down_character self)))

(fn `SetHighlight`
  (params (`Highlight?` :type Boolean))
  (`PrimitiveComponent.SetRenderCustomDepth` (`self.InteractableMesh`) `Highlight?`))

(fn `UserConstructionScript`)