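; Interactable fireplace that the player fills with logs and lights with a torch.
; A plain interaction prints a hint based on whether logs are inside.
; Adding logs removes them from the TopDownCharacter, reveals the log mesh and sets a flag.
; The torch interaction, which does not check that flag, activates particles and light, then deactivates and unregisters the fireplace and disables its interaction area collision.
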(event `Interact`
  (if (`self.LogsInFireplace?`)
    (`KismetSystemLibrary.PrintString` "I should light the logs")
    (else
      (`KismetSystemLibrary.PrintString` "I should put some logs in the fireplace"))))

(event `InteractWithLogs`
  (bind _astop_down_character (cast `/Game/TopDownBP/Blueprints/TopDownCharacter` (`GameplayStatics.GetPlayerCharacter` 0)))
  (`/Game/TopDownBP/Blueprints/TopDownCharacter.RemovePlayerLogs` _astop_down_character)
  (`SceneComponent.SetVisibility` (`self.logs`) true false)
  (set `self.LogsInFireplace?` true))

(event `InteractWithTorch`
  (`ActorComponent.Activate` (`self.ParticleSystem`) true)
  (`SceneComponent.SetVisibility` (`self.PointLight`) true false)
  (set `self.IsActive?` false)
  (bind _astop_down_character (cast `/Game/TopDownBP/Blueprints/TopDownCharacter` (`GameplayStatics.GetPlayerCharacter` 0)))
  (`/Game/TopDownBP/Blueprints/TopDownCharacter.Unregister_Interactable` _astop_down_character self)
  (`PrimitiveComponent.SetCollisionEnabled` (`self.InteractableArea`) "NoCollision"))

(fn `UserConstructionScript`
  (`parent.UserConstructionScript`))