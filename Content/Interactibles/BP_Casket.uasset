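; BP_Casket is a one-time interactable casket for inserting a body, with its mesh enlarged at BeginPlay.
; InsertBody plays a plop sound, sets the TopDownCharacter's Carrying flag to true and unregisters the casket from that character.
; It then deactivates itself, disables collision on its interaction area and runs a timeline that scales the mesh slightly larger as feedback.
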(event `self.ReceiveBeginPlay`
  (`SceneComponent.SetRelativeScale3D` (`self.InteractableMesh`) (1.25 1.25 1.25)))

(event `InsertBody`
  (`GameplayStatics.PlaySound2D` "/Game/SFX/cue_plop.cue_plop" 1.0 1.0 0.0 null null)
  (bind _astop_down_character (cast `/Game/TopDownBP/Blueprints/TopDownCharacter` (`Controller.K2_GetPawn` (`GameplayStatics.GetPlayerController` 0))))
  (set `/Game/TopDownBP/Blueprints/TopDownCharacter.Carrying?` true _astop_down_character)
  (`/Game/TopDownBP/Blueprints/TopDownCharacter.Unregister_Interactable` _astop_down_character self)
  (set `self.IsActive?` false)
  (`PrimitiveComponent.SetCollisionEnabled` (`self.InteractableArea`) "NoCollision")
  (bind (_direction _newtrack_0) (`Timeline|Timeline_0` :!via `PlayFromStart`)
    (:`Update`
      (`SceneComponent.SetRelativeScale3D` (`self.InteractableMesh`) (`KismetMathLibrary.VLerp` (1.25 1.25 1.25) (1.35 1.35 1.35) _newtrack_0)))))

(fn `UserConstructionScript`
  (`parent.UserConstructionScript`))