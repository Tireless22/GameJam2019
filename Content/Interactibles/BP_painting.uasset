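; BP_painting is an interactable painting that starts crooked and can be straightened once.
; Its construction script randomizes the mesh and a material from two arrays, then rolls the actor left or right by a fixed angle.
; RotatePainting resets the actor to zero world rotation, clears IsActive, unregisters it from the TopDownCharacter and disables the interaction area's collision.
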(event `RotatePainting`
  (`self.K2_SetActorRotation` (struct))
  (set `self.IsActive?` false)
  (bind _astop_down_character (cast `/Game/TopDownBP/Blueprints/TopDownCharacter` (`GameplayStatics.GetPlayerCharacter` 0)))
  (`/Game/TopDownBP/Blueprints/TopDownCharacter.Unregister_Interactable` _astop_down_character self)
  (`PrimitiveComponent.SetCollisionEnabled` (`self.InteractableArea`) "NoCollision"))

(fn `UserConstructionScript`
  (bind _interactablemesh (`self.InteractableMesh`))
  (`parent.UserConstructionScript`)
  (`StaticMeshComponent.SetStaticMesh` _interactablemesh (`|GetArrayItem` (`self.paintingsArray`) (`KismetMathLibrary.RandomIntegerInRange` 0 3)))
  (`PrimitiveComponent.SetMaterial` _interactablemesh 1 (`|GetArrayItem` (`self.MaterialArray`) (`KismetMathLibrary.RandomIntegerInRange` 0 3)))
  (if (== (`KismetMathLibrary.RandomIntegerInRange` 1 2) 1)
    (set `self.Rotation` 20)
    (else
      (set `self.Rotation` -20)))
  (`self.K2_SetActorRotation` (`KismetMathLibrary.MakeRotator` (`KismetMathLibrary.Conv_IntToDouble` (`self.Rotation`)))))