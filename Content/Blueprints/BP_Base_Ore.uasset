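; Breakable ore rock actor that takes damage through RockHit and shatters into a random number of BP_stone actors.
; Non-fatal hits play a pitch-varied sound, chip particles and a timeline rotation shake, with a one-time cracked mesh swap at low health.
; The shake adds to the current rotation each update; StartRotation is saved but never read.
; Random-yaw logic in the construction script is disconnected.
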(event `RockHit`
  (params (Damage :type Integer))
  (bind _health (`self.Health`))
  (bind _returnvalue (`KismetMathLibrary.MakeVector` (.x (`SceneComponent.K2_GetComponentLocation` (`self.StaticMesh`))) (.y (`SceneComponent.K2_GetComponentLocation` (`self.StaticMesh`))) (+ (.z (`SceneComponent.K2_GetComponentLocation` (`self.StaticMesh`))) 20.0)))
  (set `self.Health` (- (`self.Health`) Damage))
  (if (<= _health 0)
    (`GameplayStatics.PlaySound2D` "/Game/SFX/stone_crack_01.stone_crack_01")
    (for _ (range (+ (`KismetMathLibrary.RandomIntegerInRange` 0 3) 1))
      (`|SpawnActorFromClass` "/Game/Interactibles/Magnet_Items/BP_stone.BP_stone_C" (`KismetMathLibrary.MakeTransform` (`self.K2_GetActorLocation`)) "Undefined" "OverrideRootScale"))
    (`GameplayStatics.SpawnEmitterAtLocation` "/Game/Assets/VFX/stone_chips_big.stone_chips_big" _returnvalue)
    (`GameplayStatics.SpawnEmitterAtLocation` "/Game/Assets/VFX/stone_chips_01.stone_chips_01" _returnvalue)
    (`self.K2_DestroyActor`)
    (elif (`self.MeshSwapped?`)
      (`self.PlayShake`)
      (elif (<= _health 50)
        (set `self.MeshSwapped?` true)
        (`StaticMeshComponent.SetStaticMesh` (`self.StaticMesh`) "/Game/Assets/Meshes/stone_01_cracked.stone_01_cracked")
        (`self.PlayShake`)
        (else
          (`self.PlayShake`))))))

(event `PlayShake`
  (`GameplayStatics.PlaySound2D` "/Game/SFX/rock_01.rock_01" 1.0 (`KismetMathLibrary.RandomFloatInRange` 0.8 1.0))
  (`GameplayStatics.SpawnEmitterAtLocation` "/Game/Assets/VFX/stone_chips_01.stone_chips_01" (`KismetMathLibrary.MakeVector` (.x (`SceneComponent.K2_GetComponentLocation` (`self.StaticMesh`))) (.y (`SceneComponent.K2_GetComponentLocation` (`self.StaticMesh`))) (+ (.z (`SceneComponent.K2_GetComponentLocation` (`self.StaticMesh`))) 20.0)))
  (set `self.StartRotation` (`SceneComponent.K2_GetComponentRotation` (`self.StaticMesh`)))
  (bind (_direction _xyshake) (`Timeline|Shake` :!via `PlayFromStart`)
    (:`Update`
      (`SceneComponent.K2_SetWorldRotation` (`self.StaticMesh`) (`KismetMathLibrary.MakeRotator` (+ (.roll (`SceneComponent.K2_GetComponentRotation` (`self.StaticMesh`))) (.x _xyshake)) (+ (.pitch (`SceneComponent.K2_GetComponentRotation` (`self.StaticMesh`))) (.y _xyshake)) (.yaw (`SceneComponent.K2_GetComponentRotation` (`self.StaticMesh`)))) false false))))

(fn `UserConstructionScript`)