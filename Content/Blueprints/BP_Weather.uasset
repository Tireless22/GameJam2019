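; Weather manager that runs the day cycle and random rain showers for the top-down game.
; A looping timer, paced by UI_Clock's adjustable game speed, drives sun rotation, fog, indirect lighting and skylight from curves.
; A per-second roll starts rain, which dims and tints the sun, crossfades forest and rain audio, and spawns emitters around the player until a cooldown.
; Lightning is rolled, but its strike logic is disconnected.
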(event `FadeSun`
  ;[1 1 1] FadeSun
  (set `self.CurrentTime` (+ (`self.CurrentTime`) 0.1))
  (if (< (`self.CurrentTime`) (+ (`self.RainDuration`) 1.0))
    (if (not (<= (`self.SunIntensity`) 1.0))
      (set `self.SunIntensity` (- (`self.SunIntensity`) 0.1))
      (`LightComponent.SetIntensity` (`Light.LightComponent` (`self.Sun`)) (`self.SunIntensity`)))
    (elif (>= (`self.SunIntensity`) 3.0)
      (`KismetSystemLibrary.K2_ClearAndInvalidateTimerHandle` (stale `StartRain` _returnvalue))
      (else
        (set `self.SunIntensity` (+ (`self.SunIntensity`) 0.1))
        (`LightComponent.SetIntensity` (`Light.LightComponent` (`self.Sun`)) (`self.SunIntensity`))))))

(event `RainTimer`
  ;[1 1 1] On rain end
  (`KismetSystemLibrary.Delay` (`self.RainDuration`))
  (`|ExecutionSequence`
    (:`then_0`
      ;[1 1 1] Lerp sun color
      (bind (_direction _alpha) (`Timeline|ColorLerpEnd` :!via `PlayFromStart`)
        (:`Update`
          (`LightComponent.SetLightColor` (`Light.LightComponent` (`self.Sun`)) (`KismetMathLibrary.LinearColorLerp` (struct :`R` 0.304987 :`G` 0.423268 :`B` 0.53948 :`A` 1.0) (struct :`R` 1.0 :`G` 1.0 :`B` 1.0 :`A` 1.0) _alpha) true))))
    (:`then_1`
      ;[1 1 1] Fade out Rain sound
      (`AudioComponent.FadeOut` (`self.RainSoundRef`) 2.9 0.0)
      ;[1 1 1] invalidate timer
      (`KismetSystemLibrary.Delay` 2.0)
      (`KismetSystemLibrary.K2_ClearAndInvalidateTimerHandle` (stale `StartRain` _returnvalue_2))
      ;[1 1 1] reset rain destroyed after cooldown
      (`KismetSystemLibrary.Delay` (`self.RainCooldown`))
      (set `self.RainDestroyed?` true))
    (:`then_2`
      ;[1 1 1] Fade in forest sound
      (`KismetSystemLibrary.Delay` 2.0)
      (bind _returnvalue (`GameplayStatics.SpawnSound2D` "/Game/SFX/Forest_Loop_01.Forest_Loop_01" 1.0))
      (set `self.ForestSoundRef` _returnvalue)
      (`AudioComponent.FadeIn` (`self.ForestSoundRef`) 2.0 1.0 0.0))))

(event `StartRainSound`
  ;[1 1 1] start rain sound
  (`KismetSystemLibrary.Delay` 1.0)
  (bind _returnvalue (`GameplayStatics.SpawnSound2D` "/Game/SFX/Rain_Loop_01.Rain_Loop_01" 1.0))
  (set `self.RainSoundRef` _returnvalue)
  (`AudioComponent.FadeIn` (`self.RainSoundRef`) 2.0 1.0 0.0)
  (`AudioComponent.FadeOut` (`self.ForestSoundRef`) 2.0 0.0))

(event `StartRain`
  (set `self.RainDestroyed?` false)
  (set `self.RainDuration` (`KismetMathLibrary.RandomFloatInRange` 15.0 (`self.RainMaxDuration`)))
  (set `self.CurrentTime` 0.0)
  (`|ExecutionSequence`
    (:`then_0`
      ;[1 1 1] rain event
      (if (not (>= (`self.SecondsCounter`) 780.0))
        (bind _returnvalue (`KismetSystemLibrary.K2_SetTimerDelegate` (delegate `FadeSun`) 0.1 true)))
      (bind _returnvalue_2 (`KismetSystemLibrary.K2_SetTimerDelegate` (delegate `Rain`) 1.0 true))
      (`self.RainTimer`)
      (`self.StartRainSound`))
    (:`then_1`
      ;[1 1 1] Lerp Color on start
      (bind (_direction _alpha) (`Timeline|ColorLerpStart` :!via `PlayFromStart`)
        (:`Update`
          (`LightComponent.SetLightColor` (`Light.LightComponent` (`self.Sun`)) (`KismetMathLibrary.LinearColorLerp` (struct :`R` 1.0 :`G` 1.0 :`B` 1.0 :`A` 1.0) (struct :`R` 0.3051 :`G` 0.424356 :`B` 0.54 :`A` 1.0) _alpha) true))))))

(event `Rain`
  (bind _currentlocation (`self.CurrentLocation`))
  ;[1 1 1] rain event
  (bind _astop_down_character (cast `/Game/Blueprints/TopDownCharacter` (`GameplayStatics.GetPlayerCharacter` 0)))
  (set `self.CurrentLocation` (`SceneComponent.K2_GetComponentLocation` (`Character.Mesh` _astop_down_character)))
  (`|ExecutionSequence`
    (:`then_0`
      (`GameplayStatics.SpawnEmitterAtLocation` "/Game/Assets/VFX/Rain_Hit_Ground.Rain_Hit_Ground" (`KismetMathLibrary.MakeVector` (+ (.x _currentlocation) 700.0) (+ (.y _currentlocation) 1000.0) (`self.SpawnZHeight`))))
    (:`then_1`
      (`GameplayStatics.SpawnEmitterAtLocation` "/Game/Assets/VFX/Rain_Hit_Ground.Rain_Hit_Ground" (`KismetMathLibrary.MakeVector` (+ (.x _currentlocation) 700.0) (- (.y _currentlocation) 1000.0) (`self.SpawnZHeight`))))
    (:`then_2`
      (`GameplayStatics.SpawnEmitterAtLocation` "/Game/Assets/VFX/Rain_Hit_Ground.Rain_Hit_Ground" (`KismetMathLibrary.MakeVector` (- (.x _currentlocation) 700.0) (+ (.y _currentlocation) 1000.0) (`self.SpawnZHeight`))))
    (:`then_3`
      (`GameplayStatics.SpawnEmitterAtLocation` "/Game/Assets/VFX/Rain_Hit_Ground.Rain_Hit_Ground" (`KismetMathLibrary.MakeVector` (- (.x _currentlocation) 700.0) (- (.y _currentlocation) 1000.0) (`self.SpawnZHeight`))))))

(event `WeatherInitiator`
  ;[1 1 1] Roll for Rain
  (if (`self.RainDestroyed?`)
    (bind __ (`/Game/Blueprints/ChancePercent.Percentage` (`self.ChanceForRainPerSecond`)))
    ;[1 1 1] Roll for lightning
    (if __
      (bind ___2 (`/Game/Blueprints/ChancePercent.Percentage` (`self.ChanceForLightning`)))
      (if ___2
        (set `self.Lightning?` true)
        (else
          (set `self.Lightning?` false)))
      (`self.StartRain`))))

(event `RefreshSunFogTimer`
  (`KismetSystemLibrary.K2_ClearAndInvalidateTimerHandle` (stale _returnvalue))
  ;[1 1 1] Start update sun and fog
  (bind _returnvalue (`KismetSystemLibrary.K2_SetTimerDelegate` (delegate `StartSunAndFog`) (`self.GameTimeSpeedRef`) true :!label _label)))

(event `self.ReceiveBeginPlay`
  ;[1 1 1] Event begin play
  ;[1 1 1] Get Game Time Speed
  (bind _foundwidgets (`WidgetBlueprintLibrary.GetAllWidgetsOfClass` "/Game/UI/UI_Clock.UI_Clock_C"))
  (bind _asui_clock (cast `/Game/UI/UI_Clock` (`|GetArrayItem` _foundwidgets))
    (:`then`
      (set `self.GameTimeSpeedRef` (`/Game/UI/UI_Clock.GameTimeSpeed` _asui_clock))
      ;[1 1 1] start forest sound
      (bind _returnvalue (`GameplayStatics.SpawnSound2D` "/Game/SFX/Forest_Loop_01.Forest_Loop_01" 1.0))
      (set `self.ForestSoundRef` _returnvalue)
      ;[1 1 1] start weather
      (`KismetSystemLibrary.K2_SetTimerDelegate` (delegate `WeatherInitiator`) 1.0 true)
      (goto _label))
    (:`CastFailed`
      (`KismetSystemLibrary.PrintString` "castfail233"))))

(event `StartSunAndFog`
  ;[1 1 1] update seconds passed
  (set `self.SecondsPassed` (+ (`self.SecondsPassed`) 1.0))
  (set `self.Alpha` (/ (`self.SecondsPassed`) (`self.DayTimeInSeconds`)))
  ;[1 1 1] set fog density
  (`ExponentialHeightFogComponent.SetFogDensity` (`self.ExponentialHeightFog`) (`CurveFloat.GetFloatValue` (`self.FogDensity`) (* (`self.Alpha`) (`self.DayTimeInSeconds`))))
  ;[1 1 1] Update Sun Rotation
  (`self.K2_SetActorRotation` (`self.Sun`) (`KismetMathLibrary.MakeRotator` 0.0 (`CurveFloat.GetFloatValue` (`self.SunDirection`) (* (`self.Alpha`) (`self.DayTimeInSeconds`))) (`CurveFloat.GetFloatValue` (`self.SunDirectionZ`) (* (`self.Alpha`) (`self.DayTimeInSeconds`)))) false)
  ;[1 1 1] update skydome sun direction
  (`/Engine/EngineSky/BP_Sky_Sphere.UpdateSunDirection` (`self.Skydome`))
  ;[1 1 1] update indirect lighting intensity
  (`LightComponent.SetIndirectLightingIntensity` (`Light.LightComponent` (`self.Sun`)) (`CurveFloat.GetFloatValue` (`self.IndirectLightingIntensity`) (* (`self.Alpha`) (`self.DayTimeInSeconds`))))
  ;[1 1 1] evening fade skylight
  (`SkyLightComponent.SetIntensity` (`SkyLight.LightComponent` (`self.SkyLight`)) (`CurveFloat.GetFloatValue` (`self.SkylightIntensity`) (* (`self.Alpha`) (`self.DayTimeInSeconds`)))))

(event `/Game/Blueprints/BPI_Time.DoubleSpeed`
  ;[1 1 1] Event global time change
  (if (not (<= (`self.GameTimeSpeedRef`) 0.025))
    (set `self.GameTimeSpeedRef` (/ (`self.GameTimeSpeedRef`) 2.0))
    (`self.RefreshSunFogTimer`)))

(event `/Game/Blueprints/BPI_Time.HalfSpeed`
  ;[1 1 1] Event global time change
  (if (not (>= (`self.GameTimeSpeedRef`) 0.4))
    (set `self.GameTimeSpeedRef` (* (`self.GameTimeSpeedRef`) 2.0))
    (`self.RefreshSunFogTimer`)))

(event `/Game/Blueprints/BPI_Time.SetTime`
  (params (NewTimeInHours :type "Float (single-precision)"))
  ;[1 1 1] Event global time change
  (if (`KismetMathLibrary.InRange_FloatFloat` NewTimeInHours 0.0 26.0)
    (set `self.SecondsPassed` (* (- NewTimeInHours 6.0) 60.0))))

(fn `UserConstructionScript`)