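; Interactable blob chest that hands the player a new Blob_Character to carry.
; Three looping timelines animate it from BeginPlay: randomized roll on StaticMesh1, plus randomized pitch and a slight scale pulse on InteractableMesh.
; Interact spawns the blob with movement and collision off, attaches it to the TopDownCharacter's right-hand socket and sets it as the carried object, without checking for an existing one.
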(event `self.ReceiveBeginPlay`
  (`|ExecutionSequence`
    (:`then_0`
      (bind (_direction _newtrack_0) (`Timeline|Rotation` :!via `PlayFromStart` :!label _label)
        (:`Update`
          (`SceneComponent.K2_SetRelativeRotation` (`self.StaticMesh1`) (`KismetMathLibrary.MakeRotator` (`KismetMathLibrary.Lerp` (`self.NewVar_0`) (`self.NewVar_1`) _newtrack_0)) false false))
        (:`Finished`
          (set `self.NewVar_0` (`KismetMathLibrary.RandomFloatInRange` 10.0))
          (set `self.NewVar_1` (`KismetMathLibrary.RandomFloatInRange` -15.0 -30.0))
          (`KismetSystemLibrary.Delay` 0.2)
          (goto _label :!via `PlayFromStart`))))
    (:`then_1`
      (bind (_direction_2 _newtrack_0_2) (`Timeline|Timeline_0` :!via `PlayFromStart` :!label _label_2)
        (:`Update`
          (`SceneComponent.K2_SetRelativeRotation` (`self.InteractableMesh`) (`KismetMathLibrary.MakeRotator` 0.0 (`KismetMathLibrary.Lerp` 0.0 (`self.NewVar_3`) _newtrack_0_2)) false false))
        (:`Finished`
          (set `self.NewVar_3` (`KismetMathLibrary.RandomFloatInRange` -30.0 30.0))
          (`KismetSystemLibrary.Delay` 0.2)
          (goto _label_2 :!via `PlayFromStart`))))
    (:`then_2`
      (bind (_direction_3 _newtrack_0_3) (`Timeline|Timeline_1` :!via `PlayFromStart` :!label _label_3)
        (:`Update`
          (bind _returnvalue (`KismetMathLibrary.Lerp` 1.0 1.1 _newtrack_0_3))
          (`SceneComponent.SetRelativeScale3D` (`self.InteractableMesh`) (`KismetMathLibrary.MakeVector` _returnvalue _returnvalue _returnvalue)))
        (:`Finished`
          (`KismetSystemLibrary.Delay` 0.2)
          (goto _label_3 :!via `PlayFromStart`))))))

(event `Interact`
  (bind _astop_down_character (cast `/Game/TopDownBP/Blueprints/TopDownCharacter` (`GameplayStatics.GetPlayerCharacter` 0)))
  (set `/Game/TopDownBP/Blueprints/TopDownCharacter.Carrying?` true _astop_down_character)
  (bind _returnvalue_location (`KismetMathLibrary.BreakTransform` (`self.GetTransform` _astop_down_character)))
  (bind _returnvalue (`|SpawnActorFromClass` "/Game/TopDownBP/Blueprints/Blob_Character.Blob_Character_C" (`KismetMathLibrary.MakeTransform` _returnvalue_location) "AlwaysSpawn" "OverrideRootScale" _astop_down_character _astop_down_character))
  (set `/Game/TopDownBP/Blueprints/Blob_Character.WantsToMove?` false _returnvalue)
  (`self.SetActorEnableCollision` _returnvalue false)
  (`self.K2_AttachToComponent` _returnvalue (`Character.Mesh` _astop_down_character) "RightHand_ItemJoint" "SnapToTarget" "KeepWorld" "KeepWorld" true)
  (set `/Game/TopDownBP/Blueprints/TopDownCharacter.CarryingObject` _returnvalue _astop_down_character)
  (`self.K2_SetActorLocation` _returnvalue (+ (`self.K2_GetActorLocation` _returnvalue) (0.0 0.0 8.0)) false false)
  (`self.K2_SetActorRotation` :`self` _returnvalue))

(fn `UserConstructionScript`
  (`parent.UserConstructionScript`))